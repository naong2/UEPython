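; BP_ActorPlace is a placement tool that spawns a line of StaticMeshActors along its forward vector, spaced by Distance and driven by Count.
; The construction script previews the chosen mesh and material, moving marker meshes to the first step and line end.
; PlaceActors tags and records each spawn, falling back to a Cone mesh; AddOffset never affects spawn positions.
; RemoveActors destroys the recorded spawns, while Delete_PlacedActorAll destroys every actor tagged PlacedActor.
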(event Custom|PlaceActors
  (Utilities|Array|Clear (Variables|Default|GetCreatedActors))
  (Variables|Default|SetOffsetDelta (- "0, 0, 0" (Variables|Default|GetAddOffset)))
  (Variables|Default|SetCurrentPosition (Transformation|GetWorldLocation (Variables|Default|GetDefaultSceneRoot)))
  (for _index (range 0 (Variables|Default|GetCount))
    (bind _returnvalue (Game|SpawnActorfromClass "/Script/Engine.StaticMeshActor" (Math|Transform|MakeTransform (+ (Transformation|GetActorLocation) (* (Transformation|GetActorForwardVector) (* _index (Variables|Default|GetDistance)))) (Transformation|GetActorRotation) (Transformation|GetActorScale3D)) "Undefined" 0 0))
    (Variables|Default|SetCurrentPosition (- (Variables|Default|GetCurrentPosition) (Variables|Default|GetOffsetDelta)))
    (Utilities|FlowControl|Sequence
      (:then_0
        (bind _actor (Variables|Default|GetActor)
          (:then
            (Components|StaticMesh|SetStaticMesh (Variables|/Script/Engine.StaticMeshActor|GetStaticMeshComponent _returnvalue) _actor))
          (:else
            (Components|StaticMesh|SetStaticMesh (Variables|/Script/Engine.StaticMeshActor|GetStaticMeshComponent _returnvalue) "/Engine/BasicShapes/Cone.Cone"))))
      (:then_1
        (bind _material (Variables|Default|GetMaterial)
          (:then
            (Rendering|Material|SetMaterial (Variables|/Script/Engine.StaticMeshActor|GetStaticMeshComponent _returnvalue) 0 _material))
          (:else)))
      (:then_2
        (Variables|/Script/Engine.Actor|SetTags _returnvalue (Utilities|Array|MakeArray "PlacedActor")))
      (:then_3
        (Utilities|Array|Add (Variables|Default|GetCreatedActors) _returnvalue)))))

(event Custom|RemoveActors
  (bind _createdactors (Variables|Default|GetCreatedActors))
  (for _array_element _createdactors
    (Actor|DestroyActor _array_element))
  (Utilities|Array|Clear _createdactors))

(event Custom|Delete_PlacedActorAll
  (bind _outactors (Actor|GetAllActorswithTag "PlacedActor"))
  (for _array_element _outactors
    (Actor|DestroyActor _array_element)))

(event EventBeginPlay)

(event Collision|EventActorBeginOverlap
  (params (OtherActor :type Actor%20Object%20Reference)))

(event EventTick
  (params (DeltaSeconds :type Float%20%28single-precision%29)))

(fn ConstructionScript
  (bind _staticmesh_preview (Variables|Default|GetStaticMesh_preview))
  (bind _staticmesh_distance (Variables|Default|GetStaticMesh_Distance))
  (bind _staticmesh_offset (Variables|Default|GetStaticMesh_offset))
  (Utilities|FlowControl|Sequence
    (:then_0
      (bind _actor (Variables|Default|GetActor)
        (:then
          (Components|StaticMesh|SetStaticMesh _staticmesh_preview _actor)
          (Components|StaticMesh|SetStaticMesh _staticmesh_offset _actor)
          (Components|StaticMesh|SetStaticMesh _staticmesh_distance _actor))
        (:else)))
    (:then_1
      (bind _material (Variables|Default|GetMaterial)
        (:then
          (Rendering|Material|SetMaterial _staticmesh_preview 0 _material))
        (:else)))
    (:then_2
      (Transformation|SetWorldLocation _staticmesh_offset (+ (Transformation|GetWorldLocation (Variables|Default|GetDefaultSceneRoot)) (* (Transformation|GetActorForwardVector) (Variables|Default|GetDistance))) false false))
    (:then_3
      (Transformation|SetWorldLocation _staticmesh_distance (+ (Transformation|GetWorldLocation (Variables|Default|GetDefaultSceneRoot)) (* (Transformation|GetActorForwardVector) (* (Variables|Default|GetCount) (Variables|Default|GetDistance)))) false false))))