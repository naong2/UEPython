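; BP_Face is a Blueprint that remote-controls an iPhone face capture app over OSC, as the Live Link Face folder and addresses suggest.
; BeginPlay starts an OSC server with a bound message handler, and an OSCMessages event prints incoming addresses.
; Separate events create the client and send AR session, slate and record commands to hardcoded endpoints.
; The record events also start and stop Take Recorder, pairing phone and Unreal takes.
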(event Custom|StopRecording
  (bind _returnvalue (Class|OSCManager|ConvertStringtoOSCAddress "/RecordStop"))
  (bind _returnvalue_2 (Class|OSCManager|SetOSCMessageAddress (Utilities|Struct|MakeOSCMessage) _returnvalue))
  (Class|OSCClient|SendOSCMessage (Variables|Default|GetOSCClient) _returnvalue_2)
  (Class|TakeRecorderPanel|StopRecording (Class|TakeRecorderBlueprintLibrary|GetTakeRecorderPanel)))

(event Custom|CreateOSCServer
  (bind _returnvalue (Class|OSCManager|CreateOSCServer "192.168.1.20" 6000 true true "father" 0))
  (bind _output_get (Variables|Default|SetOSCServer _returnvalue))
  (EventDispatchers|BindEventtoOnOscMessageReceived _output_get (EventDispatchers|CreateEvent :!event Custom|OSCMessages)))

(event Custom|OSCMessages
  (params (Message :type OSC%20Message%20Structure%20%28by%20ref%29) (IPAddress :type String) (Port :type Integer))
  (bind _returnvalue (Class|OSCManager|GetOSCMessageAddress Message))
  (bind _returnvalue_2 (Class|OSCManager|GetOSCAddressFullPath _returnvalue))
  (Development|PrintString _returnvalue_2))

(event Custom|CreateClient
  (bind _returnvalue (Class|OSCManager|CreateOSCClient "192.168.1.30" 8001 "iPhone" 0))
  (Variables|Default|SetOSCClient _returnvalue))

(event Custom|ARStart
  (bind _returnvalue (Class|OSCManager|ConvertStringtoOSCAddress "/ARSessionStart"))
  (bind _returnvalue_2 (Class|OSCManager|SetOSCMessageAddress (Utilities|Struct|MakeOSCMessage) _returnvalue))
  (Class|OSCClient|SendOSCMessage (Variables|Default|GetOSCClient) _returnvalue_2))

(event Custom|Slate
  (bind _returnvalue (Class|OSCManager|ConvertStringtoOSCAddress "/Slate"))
  (bind _returnvalue_2 (Class|OSCManager|SetOSCMessageAddress (Utilities|Struct|MakeOSCMessage) _returnvalue))
  (bind _returnvalue_3 (Class|OSCManager|AddString _returnvalue_2 (Utilities|String|MakeLiteralString "Naong2")))
  (Class|OSCClient|SendOSCMessage (Variables|Default|GetOSCClient) _returnvalue_3))

(event Custom|ARStop
  (bind _returnvalue (Class|OSCManager|ConvertStringtoOSCAddress "/ARSessionStop"))
  (bind _returnvalue_2 (Class|OSCManager|SetOSCMessageAddress (Utilities|Struct|MakeOSCMessage) _returnvalue))
  (Class|OSCClient|SendOSCMessage (Variables|Default|GetOSCClient) _returnvalue_2))

(event Custom|StartRecording
  (bind _returnvalue (Class|OSCManager|ConvertStringtoOSCAddress "/RecordStart"))
  (bind _returnvalue_2 (Class|OSCManager|SetOSCMessageAddress (Utilities|Struct|MakeOSCMessage) _returnvalue))
  (bind _returnvalue_3 (Class|OSCManager|AddString _returnvalue_2 (Utilities|String|MakeLiteralString "Naong2")))
  (bind _returnvalue_4 (Class|OSCManager|AddInt32 _returnvalue_3))
  (Class|OSCClient|SendOSCMessage (Variables|Default|GetOSCClient) _returnvalue_4)
  (Class|TakeRecorderPanel|StartRecording (Class|TakeRecorderBlueprintLibrary|GetTakeRecorderPanel)))

(event EventBeginPlay
  (CallFunction|CreateOSCServer))

(event Collision|EventActorBeginOverlap
  (params (OtherActor :type Actor%20Object%20Reference)))

(event EventTick
  (params (DeltaSeconds :type Float%20%28single-precision%29)))

(fn ConstructionScript)